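; Directional light actor that drives a day/night cycle by rotating when a time change is triggered.
; A timeline, scaled by the requested hours, offsets the starting pitch; a reverse flag flips at exactly ±90 degrees pitch, switching yaw between 0 and 180.
; When the timeline finishes, exact pitch lookups in forward or reverse angle-to-hour maps give the time shown on the top-down character's HUD.
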(event `self.ReceiveBeginPlay`
  (bind _returnvalue (`GameplayStatics.GetActorOfClass` "/Game/Blueprints/BP_TopDownCharacter.BP_TopDownCharacter_C"))
  (set `self.Character` _returnvalue))

(event `TImeCycle`
  (params (TimeInHour :type "Float (double-precision)"))
  (set `self.InitialRotation` (`self.K2_GetActorRotation`))
  (bind (_direction _time_track) (`Timeline|Moving Time Timeline` :!via `PlayFromStart`)
    (:`Update`
      (`self.AdvanceTimeDayNightCycle` _time_track TimeInHour)
      (`self.ChangeRotation`))
    (:`Finished`
      (`self.UpdateCurrentTIme`))))

(fn `AdvanceTimeDayNightCycle`
  (params (`Time Track` :type "Float (double-precision)") (Hours :type "Float (double-precision)"))
  (`|ExecutionSequence`
    (:`then_0`
      (if (`self.ReverseRotation`)
        (bind _result (`/Engine/EditorBlueprintResources/StandardMacros.NegateFloat` `Time Track`)
          (:`  `
            (set `self.TimeTrack` _result)
            (set `self.Yaw` 180.0)))
        (else
          (set `self.TimeTrack` `Time Track`)
          (set `self.Yaw` 0.0))))
    (:`then_1`
      (`self.K2_SetActorRotation` (`KismetMathLibrary.MakeRotator` 0.0 (+ (.pitch (`self.InitialRotation`)) (* (`self.TimeTrack`) Hours)) (`self.Yaw`))))))

(fn `ChangeRotation`
  (if (`self.IsPitchEqual` 90.0)
    (set `self.ReverseRotation` true)
    (elif (`self.IsPitchEqual` -90.0)
      (set `self.ReverseRotation` false))))

(fn `GetHourFromAngle`
  (params (TargetMap :type "Map of Float (double-precision) to Integer (by ref)"))
  (returns (`Current Hour` :type Integer))
  (return (`BlueprintMapLibrary.Map_Find` TargetMap (.pitch (`self.K2_GetActorRotation`)))))

(fn `GetTimeOfTheDay`
  (returns (`Current Hour` :type Integer))
  (if (`self.ReverseRotation`)
    (bind _current_hour (`self.GetHourFromAngle` (`self.ReverseAnglesToHours`)))
    (return _current_hour)
    (else
      (bind _current_hour_2 (`self.GetHourFromAngle` (`self.AnglesToHours`)))
      (return _current_hour_2))))

(fn `IsPitchEqual`
  (params (`Pitch Value` :type "Float (double-precision)"))
  (returns (IsEqual :type Boolean))
  (return (== `Pitch Value` (.pitch (`self.K2_GetActorRotation`)))))

(fn `UpdateCurrentTIme`
  (bind _current_hour (`self.GetTimeOfTheDay`))
  (`/Game/Blueprints/BP_TopDownCharacter.SetTimeOnHUD` (`self.Character`) _current_hour))

(fn `UserConstructionScript`)